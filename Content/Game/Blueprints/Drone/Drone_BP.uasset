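; Player-pilotable drone pawn that spawns its HUD widget and takes possession from the player on activation, returning control on toggle.
; An Idle/Posses state enum gates activation, which first moves the drone's box above the player, and deactivation.
; Input drives floating movement, yaw, scene-capture camera pitch and a spotlight; night vision input is an empty stub.
; While possessed, Tick line-traces downward and along the camera for altitude and distance in meters.
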(event EventTick
  (params (DeltaSeconds :type Float%20%28single-precision%29))
  (bind _returnvalue (Transformation|GetActorLocation))
  (bind _scenecapturecomponent2d (Variables|Default|GetSceneCaptureComponent2D))
  (bind _returnvalue_2 (Transformation|GetWorldLocation _scenecapturecomponent2d))
  ;[1 1 1] Comment
  (switch Utilities|FlowControl|Switch|SwitchonDroneState_Enum (Variables|Default|GetDroneState_Enum)
    (:NewEnumerator1
      (Utilities|FlowControl|Sequence
        (:then_0
          (bind (_outhit _returnvalue_3) (Collision|LineTraceByChannel _returnvalue (- _returnvalue "0, 0,10000.000000") "TraceTypeQuery2" false 0 "None"))
          (Variables|Default|SetAltitude (select _returnvalue_3 (/ (.Distance (Collision|BreakHitResult _outhit)) 1e+02) -1.0)))
        (:then_1
          (bind (_outhit_2 _returnvalue_4) (Collision|LineTraceByChannel _returnvalue_2 (+ _returnvalue_2 (* (Math|Vector|GetForwardVector _scenecapturecomponent2d) 1e+04)) "TraceTypeQuery2" false 0 "None"))
          (Variables|Default|SetDistance (select _returnvalue_4 (/ (.Distance (Collision|BreakHitResult _outhit_2)) 1e+02) 0.0)))))))

(event EventBeginPlay
  (bind _asthird_person_character (Utilities|Casting|CastToThirdPersonCharacter (Game|GetPlayerCharacter 0)))
  (Variables|Default|SetPlayer%20Ref _asthird_person_character))

(event Input|ActionEvents|InputActionToggleDrone
  (params (Key :type Key%20Structure :default "None"))
  ;[1 1 1] Toggle to Player
  (:Pressed
    (CallFunction|DeactivateDrone)))

(event Input|ActionEvents|InputActionNightVision
  (params (Key :type Key%20Structure :default "None"))
  (:Pressed
    (Utilities|FlowControl|FlipFlop)))

(event Input|ActionEvents|InputActionLight
  (params (Key :type Key%20Structure :default "None"))
  ;[1 1 1] Light On/Off
  (:Pressed
    (Utilities|FlowControl|FlipFlop
      (:A
        (Development|SetHiddeninGame (Variables|Default|GetSpotLight) false false))
      (:B
        (Development|SetHiddeninGame (Variables|Default|GetSpotLight) true false)))))

(event Input|AxisEvents|InputAxisDroneUp
  (params (AxisValue :type Float%20%28single-precision%29))
  ;[1 1 1] Drone MoveUp/ MoveDown
  (Class|PawnMovementComponent|AddInputVector (Variables|Default|GetFloatingPawnMovement) (* (Math|Vector|VectorUp) AxisValue) false))

(event Input|AxisEvents|InputAxisMoveRight
  (params (AxisValue :type Float%20%28single-precision%29))
  ;[1 1 1] Drone Move Right/Left
  (Class|PawnMovementComponent|AddInputVector (Variables|Default|GetFloatingPawnMovement) (* (Transformation|GetActorRightVector) AxisValue) false))

(event Input|AxisEvents|InputAxisMoveForward
  (params (AxisValue :type Float%20%28single-precision%29))
  ;[1 1 1] Drone Move Forward/Backward
  (Class|PawnMovementComponent|AddInputVector (Variables|Default|GetFloatingPawnMovement) (* (Transformation|GetActorForwardVector) AxisValue) false))

(event Input|AxisEvents|InputAxisTurn
  (params (AxisValue :type Float%20%28single-precision%29))
  ;[1 1 1] Drone Turn
  (Pawn|Input|AddControllerYawInput AxisValue))

(event Input|AxisEvents|InputAxisLookUp
  (params (AxisValue :type Float%20%28single-precision%29))
  ;[1 1 1] Drone LookUp
  (Transformation|SetRelativeRotation (Variables|Default|GetSceneCaptureComponent2D) (Math|Rotator|MakeRotator 0.0 (Math|Float|Clamp(Float) (+ (* AxisValue -1.0) (.pitch (Variables|/Script/Engine.SceneComponent|GetRelativeRotation (Variables|Default|GetSceneCaptureComponent2D)))) -1.8e+02 3e+01) 0.0) false false))

(fn ConstructionScript)

(fn ActivateDrone
  (params (Interactor :type Character%20Object%20Reference))
  ;[1 1 1] Activate Drone
  (CallFunction|SetDroneLocation)
  (switch Utilities|FlowControl|Switch|SwitchonDroneState_Enum (Variables|Default|GetDroneState_Enum)
    (:NewEnumerator0
      (bind _output_get (Variables|Default|SetInteractor Interactor))
      (bind _asplayer_controller (Utilities|Casting|CastToPlayerController (Pawn|GetController _output_get)))
      (bind _output_get_2 (Variables|Default|SetPlayer%20Controller _asplayer_controller))
      (bind _returnvalue (UserInterface|CreateWidget "/Game/Game/Blueprints/Drone/Drone_Widget_BP.Drone_Widget_BP_C" _output_get_2))
      (bind _output_get_3 (Variables|Default|SetDrone%20Screen%20Widget _returnvalue))
      (UserInterface|Viewport|AddtoViewport _output_get_3 0)
      (Pawn|Possess (Variables|Default|GetPlayer%20Controller) self)
      (Variables|Default|SetDroneState_Enum "NewEnumerator1"))))

(fn DeactivateDrone
  ;[1 1 1] Deactivate Drone
  (switch Utilities|FlowControl|Switch|SwitchonDroneState_Enum (Variables|Default|GetDroneState_Enum)
    (:NewEnumerator1
      (Pawn|Possess (Pawn|GetController) (Variables|Default|GetInteractor))
      (Variables|Default|SetInteractor 0)
      (Widget|RemovefromParent (Variables|Default|GetDrone%20Screen%20Widget))
      (Variables|Default|SetDroneState_Enum "NewEnumerator0"))))

(fn SetDroneLocation
  (bind _player_ref (Variables|Default|GetPlayer%20Ref))
  (bind _returnvalue (Transformation|GetActorLocation _player_ref))
  (Transformation|SetWorldLocation (Variables|Default|GetBox) (Math|Vector|MakeVector (.x _returnvalue) (.y _returnvalue) (+ (.z _returnvalue) 8e+01)) false false))

(fn GetAltitudeinMeters
  (return (Variables|Default|GetAltitude)))

(fn GetDistanceinMeters
  (return (Variables|Default|GetDistance)))