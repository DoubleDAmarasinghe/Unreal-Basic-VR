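; VR handgun that the player grabs and fires with either hand.
; Grab, within the Grip sphere, snaps it to that hand's socket and enables firing; Release detaches it and restores physics.
; Per-hand fire events play sound and muzzle effect, then line trace from the muzzle, spawning a projectile only on a hit.
; Empty ammo plays a dry-fire sound; firing never decrements AmmoCount here, and recoil nodes are disconnected.
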(event Custom|HandGunFireRight
  (bind _staticmesh (Variables|Default|GetStaticMesh))
  (bind _staticmesh_2 (Variables|Default|GetStaticMesh))
  (bind _returnvalue (Transformation|GetSocketLocation _staticmesh_2 "MuzzleLocation"))
  ;[1 1 1] HandGun Fire Right Hand
  (if (Math|Boolean|ANDBoolean (Variables|Default|GetCanFireRight) (> (Variables|Default|GetAmmoCount) 0) (== (Variables|/Game/VRTemplate/Blueprints/NewVR/NewVRCharacter.NewVRCharacter_C|GetRightGrabactor (Variables|Default|GetVRPlayerRef)) self))
    (bind _returnvalue_2 (Audio|CreateSound2D "/Game/Game/Sounds/SHOT2.SHOT2" 1.0 1.0 0.0 0))
    (Audio|Components|Audio|Play _returnvalue_2 0.0)
    (bind _returnvalue_3 (Effects|SpawnEmitteratLocation "/Engine/Tutorial/SubEditors/TutorialAssets/TutorialParticleSystem.TutorialParticleSystem" (Transformation|GetSocketLocation _staticmesh "MuzzleLocation") (Transformation|GetSocketRotation _staticmesh "MuzzleLocation") "0.500000,0.500000,0.500000"))
    (bind (_outhit _returnvalue_4) (Collision|LineTraceByChannel _returnvalue (+ _returnvalue (* (Math|Vector|GetRightVector (Transformation|GetWorldRotation _staticmesh_2)) 5e+03)) "TraceTypeQuery1" false 0 "ForDuration"))
    (if _returnvalue_4
      (Game|SpawnActorfromClass "/Game/VRTemplate/Blueprints/Projectile.Projectile_C" (Math|Transform|MakeTransform _returnvalue (Math|Rotator|FindLookatRotation (.Location (Collision|BreakHitResult _outhit)) (.TraceEnd (Collision|BreakHitResult _outhit)))) "AlwaysSpawn" 0 (Variables|Default|GetVRPlayerRef))
      (Utilities|FlowControl|Delay 0.1)
      (Components|DestroyComponent _returnvalue_3))
    (else
      ;;[1 1 1] If Doesn't Have Ammo
      (if (and (Variables|Default|GetCanFireRight) (== (Variables|Default|GetAmmoCount) 0))
        (bind _returnvalue_5 (Audio|CreateSound2D "/Game/Game/Sounds/EmptyRound.EmptyRound" 1.0 1.0 0.0 0))
        (Audio|Components|Audio|Play _returnvalue_5 0.0)))))

(event Custom|HandGunFireLeft
  (bind _staticmesh (Variables|Default|GetStaticMesh))
  (bind _staticmesh_2 (Variables|Default|GetStaticMesh))
  (bind _returnvalue (Transformation|GetSocketLocation _staticmesh_2 "MuzzleLocation"))
  ;[1 1 1] HandGun Fire Right Hand
  (if (Math|Boolean|ANDBoolean (Variables|Default|GetCanFireLeft) (> (Variables|Default|GetAmmoCount) 0) (== (Variables|/Game/VRTemplate/Blueprints/NewVR/NewVRCharacter.NewVRCharacter_C|GetLeftGrabActor (Variables|Default|GetVRPlayerRef)) self))
    (bind _returnvalue_2 (Audio|CreateSound2D "/Game/Game/Sounds/SHOT2.SHOT2" 1.0 1.0 0.0 0))
    (Audio|Components|Audio|Play _returnvalue_2 0.0)
    (bind _returnvalue_3 (Effects|SpawnEmitteratLocation "/Engine/Tutorial/SubEditors/TutorialAssets/TutorialParticleSystem.TutorialParticleSystem" (Transformation|GetSocketLocation _staticmesh "MuzzleLocation") (Transformation|GetSocketRotation _staticmesh "MuzzleLocation") "0.500000,0.500000,0.500000"))
    (bind (_outhit _returnvalue_4) (Collision|LineTraceByChannel _returnvalue (+ _returnvalue (* (Math|Vector|GetRightVector (Transformation|GetWorldRotation _staticmesh_2)) 5e+03)) "TraceTypeQuery1" false 0 "ForDuration"))
    (if _returnvalue_4
      (Game|SpawnActorfromClass "/Game/VRTemplate/Blueprints/Projectile.Projectile_C" (Math|Transform|MakeTransform _returnvalue (Math|Rotator|FindLookatRotation (.Location (Collision|BreakHitResult _outhit)) (.TraceEnd (Collision|BreakHitResult _outhit)))) "AlwaysSpawn" 0 (Variables|Default|GetVRPlayerRef))
      (Utilities|FlowControl|Delay 0.1)
      (Components|DestroyComponent _returnvalue_3))
    (else
      ;;[1 1 1] If Doesn't Have Ammo
      (if (and (Variables|Default|GetCanFireLeft) (== (Variables|Default|GetAmmoCount) 0))
        (bind _returnvalue_5 (Audio|CreateSound2D "/Game/Game/Sounds/EmptyRound.EmptyRound" 1.0 1.0 0.0 0))
        (Audio|Components|Audio|Play _returnvalue_5 0.0)))))

(event EventBeginPlay
  (bind _returnvalue (Actor|GetActorOfClass "/Game/VRTemplate/Blueprints/NewVR/NewVRCharacter.NewVRCharacter_C"))
  (Variables|Default|SetVRPlayerRef _returnvalue))

(event EventGrab
  (params (MotionController :type Motion%20Controller%20Component%20Object%20Reference))
  (bind _grip (Variables|Default|GetGrip))
  ;[0.02745 0.3608 1] Interface Grab Action
  (if (<= (Math|Vector|Distance(Vector) (Transformation|GetWorldLocation MotionController) (Transformation|GetWorldLocation _grip)) (Variables|/Script/Engine.SphereComponent|GetSphereRadius _grip))
    (bind _output_get (Variables|Default|SetMainGrip MotionController))
    (Physics|SetSimulatePhysics (Variables|Default|GetStaticMesh) false)
    (Utilities|FlowControl|Sequence
      (:then_0
        (if (== _output_get (Variables|/Game/VRTemplate/Blueprints/NewVR/NewVRCharacter.NewVRCharacter_C|GetMotionControllerRight (Variables|Default|GetVRPlayerRef)))
          (Transformation|AttachComponentToComponent (Variables|/Game/VRTemplate/Blueprints/NewVR/NewVRCharacter.NewVRCharacter_C|GetSkeletalMeshRight (Variables|Default|GetVRPlayerRef)) "RightHandGunHolder" "SnapToTarget" "SnapToTarget" "KeepRelative" true)
          (Variables|Default|SetCanFireRight true)))
      (:then_1
        (if (== _output_get (Variables|/Game/VRTemplate/Blueprints/NewVR/NewVRCharacter.NewVRCharacter_C|GetMotionControllerLeft (Variables|Default|GetVRPlayerRef)))
          (Transformation|AttachComponentToComponent (Variables|/Game/VRTemplate/Blueprints/NewVR/NewVRCharacter.NewVRCharacter_C|GetSkeletalMeshLeft (Variables|Default|GetVRPlayerRef)) "LeftHandGunHolder" "SnapToTarget" "SnapToTarget" "KeepRelative" true)
          (Variables|Default|SetCanFireLeft true))))))

(event EventRelease
  (params (Motioncontroller :type Motion%20Controller%20Component%20Object%20Reference))
  ;[0.02745 0.3608 1] Interface Release Acrion
  (if (== Motioncontroller (Variables|Default|GetMainGrip))
    (Physics|SetSimulatePhysics (Variables|Default|GetStaticMesh) true)
    (Variables|Default|SetMainGrip 0)
    (Transformation|DetachFromActor "KeepWorld" "KeepWorld" "KeepWorld")
    (Variables|Default|SetCanFireLeft false)
    (Variables|Default|SetCanFireRight false)))

(fn ConstructionScript)