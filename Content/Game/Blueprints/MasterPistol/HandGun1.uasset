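; HandGun1 is a VR pistol that the player can grab and release with either hand through interface events.
; Grab checks that the controller is within the Grip sphere radius, stores it as MainGrip, then snap-attaches to that hand mesh's holder socket on the cached NewVRCharacter.
; Release detaches, keeping world transform, only for the holding controller.
; FireRight is a placeholder that prints a debug string, regardless of whether the gun is held.
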(event EventBeginPlay
  (bind _returnvalue (Actor|GetActorOfClass "/Game/VRTemplate/Blueprints/NewVR/NewVRCharacter.NewVRCharacter_C"))
  (Variables|Default|SetVRPlayerRef _returnvalue))

(event EventGrab
  (params (MotionController :type Motion%20Controller%20Component%20Object%20Reference))
  (bind _grip (Variables|Default|GetGrip))
  ;[0.02745 0.3608 1] Interface Grab Action
  (if (<= (Math|Vector|Distance(Vector) (Transformation|GetWorldLocation MotionController) (Transformation|GetWorldLocation _grip)) (Variables|/Script/Engine.SphereComponent|GetSphereRadius _grip))
    (bind _output_get (Variables|Default|SetMainGrip MotionController))
    (Utilities|FlowControl|Sequence
      (:then_0
        (if (== _output_get (Variables|/Game/VRTemplate/Blueprints/NewVR/NewVRCharacter.NewVRCharacter_C|GetMotionControllerRight (Variables|Default|GetVRPlayerRef)))
          (Transformation|AttachComponentToComponent (Variables|/Game/VRTemplate/Blueprints/NewVR/NewVRCharacter.NewVRCharacter_C|GetSkeletalMeshRight (Variables|Default|GetVRPlayerRef)) "RightHolder" "SnapToTarget" "SnapToTarget" "KeepRelative" true)))
      (:then_1
        (if (== _output_get (Variables|/Game/VRTemplate/Blueprints/NewVR/NewVRCharacter.NewVRCharacter_C|GetMotionControllerLeft (Variables|Default|GetVRPlayerRef)))
          (Transformation|AttachComponentToComponent (Variables|/Game/VRTemplate/Blueprints/NewVR/NewVRCharacter.NewVRCharacter_C|GetSkeletalMeshLeft (Variables|Default|GetVRPlayerRef)) "LeftHolder" "SnapToTarget" "SnapToTarget" "KeepRelative" true))))))

(event EventRelease
  (params (Motioncontroller :type Motion%20Controller%20Component%20Object%20Reference))
  ;[0.02745 0.3608 1] Interface Release Acrion
  (if (== Motioncontroller (Variables|Default|GetMainGrip))
    (Variables|Default|SetMainGrip 0)
    (Transformation|DetachFromActor "KeepWorld" "KeepWorld" "KeepWorld")))

(event Input|ActionEvents|InputActionFireRight
  (params (Key :type Key%20Structure :default "None"))
  (:Pressed
    (Development|PrintString "Hello")))

(fn ConstructionScript)