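; TargetSpawner Blueprint that spawns Target actors at randomly chosen locations and tracks a Point total.
; Its SpawnTarget event increases Point by a fixed amount, then spawns a Target using the transform of a random pick from seven target point references.
; The file contains no trigger for SpawnTarget, and the construction script is empty.
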(event Custom|SpawnTarget
  (Variables|Default|SetPoint (+ (Variables|Default|GetPoint) 5.0))
  (Game|SpawnActorfromClass "/Game/Game/Blueprints/Target.Target_C" (Transformation|GetActorTransform (Utilities|Array|Get(acopy) (Utilities|Array|MakeArray (Variables|Default|Gettargetpoint1) (Variables|Default|Gettargetpoint2) (Variables|Default|Gettargetpoint3) (Variables|Default|Gettargetpoint4) (Variables|Default|Gettargetpoint5) (Variables|Default|Gettargetpoint6) (Variables|Default|Gettargetpoint7)) (Math|Random|RandomIntegerinRange 0 6))) "Undefined" 0 0))

(fn ConstructionScript)